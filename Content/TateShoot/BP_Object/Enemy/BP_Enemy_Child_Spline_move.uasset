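; Child enemy Blueprint for the TateShoot shooter that travels along a spline while firing at the player.
; On BeginPlay, a looping timer spawns BP_Enemy_Projectile at the enemy's location every second, rotated toward player pawn 0.
; A timeline started alongside it scales its Alpha by spline length to place the actor at that world-space point along the spline.
; The construction script only calls the parent's.
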(event Custom|SpawnProjectile
  (bind _returnvalue (Transformation|GetActorLocation))
  ;[1 1 1] 敵が弾を撃つ
  (Game|SpawnActorfromClass "/Game/TateShoot/BP_Object/Enemy/BP_Enemy_Projectile.BP_Enemy_Projectile_C" (Math|Transform|MakeTransform _returnvalue (Math|Rotator|FindLookatRotation _returnvalue (Transformation|GetActorLocation (Game|Player|GetPlayerPawn 0))) "1,1,1") "Undefined" 0 0))

(event EventBeginPlay
  (bind _target (Variables|Default|GetTarget))
  (Utilities|FlowControl|Sequence
    (:then_0
      ;[1 1 1] 敵が弾を撃つ
      (Utilities|Time|SetTimerbyEvent (delegate Custom|SpawnProjectile) 1.0 true))
    (:then_1
      ;[1 1 1] スプラインに沿って動く
      (bind _alpha (Timeline|Timeline_Spline PlayFromStart)
        (:Update
          (Transformation|SetActorTransform (Math|Transform|MakeTransform (Spline|GetLocationatDistanceAlongSpline _target (* (Spline|GetSplineLength _target) _alpha) "World") "0, 0, 0" "1,1,1")))))))

(fn ConstructionScript
  (|CallParentFunction))