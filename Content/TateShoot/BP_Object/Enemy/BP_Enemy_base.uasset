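; BP_Enemy_base is an enemy base class that handles taking damage and dying in the TateShoot game.
; AnyDamage subtracts damage from HP and prints the remaining value.
; At zero HP it disables collision, spawns a death actor and one of two randomly chosen item pickups, plays a sound, and destroys itself.
; Before destruction it reports 100 points to the GameState through an interface message.
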(event Game|Damage|EventAnyDamage
  (params (Damage :type Float%20%28single-precision%29) (DamageType :type Damage%20Type%20Object%20Reference) (InstigatedBy :type Controller%20Object%20Reference) (DamageCauser :type Actor%20Object%20Reference))
  ;[1 1 1] 敵がダメージを食らう
  (bind _output_get (Variables|Default|SetHP (- (Variables|Default|GetHP) Damage)))
  (Development|PrintString (Utilities|String|ToString(Float) _output_get))
  (if (not (> _output_get 0.0))
    ;[1 1 1] HPがゼロ以下になった時の処理
    (Collision|SetActorEnableCollision false)
    (Game|SpawnActorfromClass "/Game/TateShoot/FX/BP_Enemy_Death.BP_Enemy_Death_C" (Transformation|GetActorTransform) "Undefined" 0 0)
    (Game|SpawnActorfromClass (select (Math|Random|RandomBool) "/Game/TateShoot/BP_Object/Item/BP_Item_Child_B.BP_Item_Child_B_C" "/Game/TateShoot/BP_Object/Item/BP_Item_Child_A.BP_Item_Child_A_C") (Math|Transform|MakeTransform (Transformation|GetActorLocation) "0, 0, 0" "1,1,1") "Undefined" 0)
    (Audio|SpawnSound2D "/Game/TateShoot/Sound/SE_Death.SE_Death" 1.0 1.5 0.0 0)
    (Class|BPIGameState|BPIGameStateScoreCountUp(Message) (Game|GetGameState) 100)
    (Actor|DestroyActor)))

(fn ConstructionScript)