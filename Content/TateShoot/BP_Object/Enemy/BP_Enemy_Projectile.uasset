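; BP_Enemy_Projectile is an enemy bullet in the TateShoot game that resolves its hits through a sphere overlap event.
; Overlapping an actor tagged Player applies damage, then destroys the projectile.
; Overlapping an actor tagged Bom spawns BP_Enemy_Death and a BP_Item_Child pickup at the projectile's location before destroying it.
; Any other overlap simply destroys it, and the graphs contain no movement logic.
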(event OnComponentBeginOverlap(Sphere)
  (params (OverlappedComponent :type Primitive%20Component%20Object%20Reference) (OtherActor :type Actor%20Object%20Reference) (OtherComp :type Primitive%20Component%20Object%20Reference) (OtherBodyIndex :type Integer) (bFromSweep :type Boolean) (SweepResult :type Hit%20Result%20Structure%20%28by%20ref%29))
  (if (Actor|ActorHasTag OtherActor "Player")
    (Game|Damage|ApplyDamage OtherActor 1.0 0 0)
    (Actor|DestroyActor)
    (elif (Actor|ActorHasTag OtherActor "Bom")
      (Game|SpawnActorfromClass "/Game/TateShoot/FX/BP_Enemy_Death.BP_Enemy_Death_C" (Transformation|GetActorTransform) "Undefined" 0 0)
      (Game|SpawnActorfromClass "/Game/TateShoot/BP_Object/Item/BP_Item_Child_C.BP_Item_Child_C_C" (Math|Transform|MakeTransform (Transformation|GetActorLocation) "0, 0, 0" "1,1,1") "Undefined" 0 0)
      (Actor|DestroyActor)
      (else
        (Actor|DestroyActor)))))

(fn ConstructionScript)