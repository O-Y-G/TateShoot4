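; Player pawn for a 2D vertical shooter, handling axis movement, shooting, bombs and death with respawn.
; Holding Shoot runs a looping timer that spawns projectiles; bombs consume stock and grant temporary invincibility behind a DoOnce lock.
; Damage while vulnerable decrements Life, spawns a death effect, hides and disables the player, then respawns it at the BeginPlay position with a darkened sprite during brief invincibility.
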(event Custom|ShootLoop
  ;[1 1 1] ショット処理
  (Game|SpawnActorfromClass "/Game/TateShoot/BP_Object/BP_Player_Projectile.BP_Player_Projectile_C" (Transformation|GetActorTransform) "Undefined" 0 0)
  (Audio|SpawnSound2D "/Game/TateShoot/Sound/SE_Shoot.SE_Shoot" 1.0 1.0 0.0 0))

(event Game|Damage|EventAnyDamage
  (params (Damage :type Float%20%28single-precision%29) (DamageType :type Damage%20Type%20Object%20Reference) (InstigatedBy :type Controller%20Object%20Reference) (DamageCauser :type Actor%20Object%20Reference))
  ;[1 1 1] 死亡処理
  (if (not (Variables|Default|GetbInvincible))
    (bind _result (Math|Integer|DecrementInt (Variables|Default|GetLife))
      (:%20%20
        (Development|PrintString (Utilities|String|ToString(Integer) _result))
        (Variables|Default|SetbInvincible true)
        (Variables|Default|SetbDeath true)
        (Input|DisableInput 0)
        (Collision|SetActorEnableCollision false)
        (Game|SpawnActorfromClass "/Game/TateShoot/FX/BP_Player_Death.BP_Player_Death_C" (Transformation|GetActorTransform) "Undefined" 0 0)
        (Audio|SpawnSound2D "/Game/TateShoot/Sound/SE_Death.SE_Death" 1.0 1.0 0.0 0)
        (Development|SetHiddeninGame (Variables|Default|GetScene) true true)
        (Utilities|Time|ClearandInvalidateTimerbyHandle (Variables|Default|GetShootTimer))
        (Utilities|FlowControl|Delay 2.0)
        (Transformation|SetActorLocation (Variables|Default|GetStartPos) false false)
        (Development|SetHiddeninGame (Variables|Default|GetScene) false true)
        (Variables|Default|SetbDeath false)
        (Collision|SetActorEnableCollision true)
        (Input|EnableInput 0)
        (Sprite|SetSpriteColor (Variables|Default|GetPaperSprite) "(R=0.000000,G=0.000000,B=0.000000,A=1.000000)")
        (Utilities|FlowControl|Delay 2.0)
        (Variables|Default|SetbInvincible false)
        (Sprite|SetSpriteColor (Variables|Default|GetPaperSprite) "(R=1.000000,G=1.000000,B=1.000000,A=1.000000)")))))

(event EventBeginPlay
  ;[1 1 1] スタート位置を記憶
  (Variables|Default|SetStartPos (Transformation|GetActorLocation)))

(event Input|ActionEvents|InputActionShoot
  (params (Key :type Key%20Structure :default "None"))
  ;[1 1 1] ショット処理
  (:Pressed
    (if (not (Variables|Default|GetbDeath))
      (bind _returnvalue (Utilities|Time|SetTimerbyEvent (delegate Custom|ShootLoop) 0.1 true))
      (Variables|Default|SetShootTimer _returnvalue)
      (CallFunction|ShootLoop)))
  (:Released
    (Utilities|Time|ClearandInvalidateTimerbyHandle (Variables|Default|GetShootTimer))))

(event Input|ActionEvents|InputActionBom
  (params (Key :type Key%20Structure :default "None"))
  (bind _bom (Variables|Default|GetBom))
  ;[1 1 1] ボム処理
  (:Pressed
    (if (not (Variables|Default|GetbDeath))
      (if (> _bom 0)
        (Utilities|FlowControl|DoOnce false :!label _label
          (:Completed
            (Math|Integer|DecrementInt _bom
              (:%20%20
                (Variables|Default|SetbInvincible true)
                (Game|SpawnActorfromClass "/Game/TateShoot/BP_Object/BP_Player_Bom.BP_Player_Bom_C" (Transformation|GetActorTransform) "Undefined" 0 0)
                (Audio|PlaySound2D "/Game/TateShoot/Sound/SE_Bom.SE_Bom" 1.0 1.0 0.0 0 0)
                (Utilities|FlowControl|Delay 5.0)
                (Variables|Default|SetbInvincible false)
                (goto _label Reset)))))))))

(event Input|AxisEvents|InputAxisMoveForward
  (params (AxisValue :type Float%20%28single-precision%29))
  ;[1 1 1] 上下移動
  (Pawn|Input|AddMovementInput "0,1.000000,0.000000" AxisValue false))

(event Input|AxisEvents|InputAxisMoveRight
  (params (AxisValue :type Float%20%28single-precision%29))
  ;[1 1 1] 左右移動
  (Pawn|Input|AddMovementInput "1.000000, 0, 0" AxisValue false))

(fn ConstructionScript)