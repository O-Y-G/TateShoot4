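; BP_Item_Child_A is a score pickup item for the TateShoot game, derived from a parent item Blueprint.
; On overlap with an actor tagged Player, it sends a 50-point score message to the GameState through an interface, plays a 2D pickup sound and destroys itself.
; Overlaps with other actors destroy it only while its ProjectileMovement velocity points along positive Y.
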(event EventBeginPlay
  (|CallParentFunction) ; このノードは無効になっているため呼び出せません。\n機能をビルドするにはピンをドラッグしてください。
)

(event Collision|EventActorBeginOverlap
  (params (OtherActor :type Actor%20Object%20Reference))
  (if (Actor|ActorHasTag OtherActor "Player")
    (Class|BPIGameState|BPIGameStateScoreCountUp(Message) (Game|GetGameState) 50)
    (Audio|SpawnSound2D "/Game/TateShoot/Sound/SE_Item.SE_Item" 1.0 1.0 0.0 0)
    (Actor|DestroyActor)
    (elif (> (.y (Variables|/Script/Engine.MovementComponent|GetVelocity (Variables|Default|GetProjectileMovement))) 0.0)
      (Actor|DestroyActor))))

(fn ConstructionScript
  (|CallParentFunction))