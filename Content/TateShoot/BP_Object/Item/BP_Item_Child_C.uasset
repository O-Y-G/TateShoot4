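; Score pickup item, a child item Blueprint, that awards points when the player touches it.
; An outer homing sphere detects the player and switches the projectile movement to home in on the overlapping component.
; The main sphere's overlap with the player sends the score to the GameState through an interface message, plays a 2D sound and destroys the item.
; Other overlaps destroy it only while it moves in positive Y.
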(event OnComponentBeginOverlap(Sphere)
  (params (OverlappedComponent :type Primitive%20Component%20Object%20Reference) (OtherActor :type Actor%20Object%20Reference) (OtherComp :type Primitive%20Component%20Object%20Reference) (OtherBodyIndex :type Integer) (bFromSweep :type Boolean) (SweepResult :type Hit%20Result%20Structure%20%28by%20ref%29))
  (if (Actor|ActorHasTag OtherActor "Player")
    (Class|BPIGameState|BPIGameStateScoreCountUp(Message) (Game|GetGameState) 50)
    (Audio|SpawnSound2D "/Game/TateShoot/Sound/SE_Item.SE_Item" 1.0 1.0 0.0 0)
    (Actor|DestroyActor)
    (elif (> (.y (Variables|/Script/Engine.MovementComponent|GetVelocity (Variables|Default|GetProjectileMovement))) 0.0)
      (Actor|DestroyActor))))

(event OnComponentBeginOverlap(Sphere_Homing)
  (params (OverlappedComponent :type Primitive%20Component%20Object%20Reference) (OtherActor :type Actor%20Object%20Reference) (OtherComp :type Primitive%20Component%20Object%20Reference) (OtherBodyIndex :type Integer) (bFromSweep :type Boolean) (SweepResult :type Hit%20Result%20Structure%20%28by%20ref%29))
  (bind _projectilemovement (Variables|Default|GetProjectileMovement))
  (if (Actor|ActorHasTag OtherActor "Player")
    (Variables|/Script/Engine.ProjectileMovementComponent|SetbIsHomingProjectile _projectilemovement true)
    (Variables|/Script/Engine.ProjectileMovementComponent|SetHomingAccelerationMagnitude _projectilemovement 5e+03)
    (Variables|/Script/Engine.ProjectileMovementComponent|SetHomingTargetComponent _projectilemovement OtherComp)
    (Variables|/Script/Engine.ProjectileMovementComponent|SetMaxSpeed _projectilemovement 6e+02)))

(event EventBeginPlay
  (|CallParentFunction) ; このノードは無効になっているため呼び出せません。\n機能をビルドするにはピンをドラッグしてください。
)

(fn ConstructionScript
  (|CallParentFunction))